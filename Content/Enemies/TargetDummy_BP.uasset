(event Custom|OnTakeAnyDamage_Event
  (params (DamagedActor :type Actor%20Object%20Reference) (Damage :type Float%20%28single-precision%29) (DamageType :type Damage%20Type%20Object%20Reference) (InstigatedBy :type Controller%20Object%20Reference) (DamageCauser :type Actor%20Object%20Reference))
  (EventDispatchers|BindEventtoOnTakeAnyDamage (delegate Custom|OnTakeAnyDamage_Event))
  (Variables|Default|Sethealth (- 0.0 (Variables|Default|Gethealth)))
  (Development|PrintString (Utilities|String|ToString(Float) (Variables|Default|Gethealth))))

(event EventTick
  (params (DeltaSeconds :type Float%20%28single-precision%29))
  (CallFunction|CheckHealth))

(fn ConstructionScript)

(fn CheckHealth
  (if (<= (Variables|Default|Gethealth) 0.0)
    (Actor|DestroyActor)))